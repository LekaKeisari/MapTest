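; BP_WorldMap is an actor that displays a world map as manually placed widget tiles forming a seamless image.
; On construction and BeginPlay it loops over root child WidgetComponents, assigning entries from a Textures array to each WBP_Map image by child index.
; The construction pass offsets that index by minus one, while BeginPlay does not.
; A GeoReferencing placement path remains disconnected because its real-world scale was unusable.
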(event `self.ReceiveBeginPlay`
  ;[1 1 1] Tried setting the map images via coordinates but the plugin is in real world scale and no option to scale down exists. Had to place them manually to create a seamless map
  (for (_array_element _array_index) (`SceneComponent.GetChildrenComponents` (`self.DefaultSceneRoot`) false)
    (bind _aswidget_component (cast `WidgetComponent` _array_element))
    (bind _aswbp_map (cast `/Game/WBP_Map` (`WidgetComponent.GetWidget` _aswidget_component)))
    (`self.SetTexture` (`|GetArrayItem` (`self.Textures`) _array_index) _aswbp_map)))

(fn `SetTexture`
  (params (Texture :type "Texture2D Object Reference") (Target :type "/Game/WBP_Map Object Reference"))
  (`Image.SetBrushFromTexture` (`/Game/WBP_Map.Image1` Target) Texture false))

(fn `UserConstructionScript`
  (for (_array_element _array_index) (`SceneComponent.GetChildrenComponents` (`self.DefaultSceneRoot`) false)
    (bind _aswidget_component (cast `WidgetComponent` _array_element))
    (bind _aswbp_map (cast `/Game/WBP_Map` (`WidgetComponent.GetWidget` _aswidget_component)))
    (`self.SetTexture` (`|GetArrayItem` (`self.Textures`) (+ _array_index -1)) _aswbp_map)))