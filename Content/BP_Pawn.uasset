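; BP_Pawn is a player pawn for picking points on a georeferenced map with the mouse.
; On BeginPlay it adds the input mapping, shows the cursor, caches the HUD overlay and the BP_MapMarker actor, and sets a low screen resolution.
; On click it traces under the cursor, moves the marker to the hit, and uses the GeoReferencing system to display that point's longitude and latitude in the overlay.
; The zoom input is an empty stub.
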(event `self.ReceiveBeginPlay`
  (bind _returnvalue (`GameplayStatics.GetPlayerController` 0))
  (`EnhancedInputSubsystemInterface.AddMappingContext` (pcsubsystem `EnhancedInputLocalPlayerSubsystem` (`GameplayStatics.GetPlayerController` 0)) "/Game/Input/IMC_Default.IMC_Default" 0 (struct))
  (set `PlayerController.bShowMouseCursor` true _returnvalue)
  (bind _asbp_hud (cast `/Game/BP_HUD` (`PlayerController.GetHUD` _returnvalue)))
  (set `self.Hud Overlay` (`/Game/BP_HUD.HudOverlay` _asbp_hud))
  (bind _returnvalue_2 (`GameplayStatics.GetActorOfClass` "/Game/BP_MapMarker.BP_MapMarker_C"))
  (set `self.MapMarker` _returnvalue_2)
  (bind _returnvalue_3 (`GameUserSettings.GetGameUserSettings`))
  (`GameUserSettings.SetScreenResolution` _returnvalue_3 (make `IntPoint` 800 600)))

(event `EnhancedInput|/Game/Input/IA_Zoom`
  (params (ActionValue :type "Float (double-precision)") (ElapsedSeconds :type "Float (double-precision)") (TriggeredSeconds :type "Float (double-precision)") (InputAction :type "InputAction Object Reference" :default "/Game/Input/IA_Zoom.IA_Zoom")))

(event `EnhancedInput|/Game/Input/IA_Click`
  (params (ActionValue :type Boolean) (ElapsedSeconds :type "Float (double-precision)") (TriggeredSeconds :type "Float (double-precision)") (InputAction :type "InputAction Object Reference" :default "/Game/Input/IA_Click.IA_Click"))
  (bind _hud_overlay (`self.Hud Overlay`))
  (bind (_bblockinghit _binitialoverlap _time _distance _location) (`GameplayStatics.BreakHitResult` (`PlayerController.GetHitResultUnderCursorByChannel` (`GameplayStatics.GetPlayerController` 0) "TraceTypeQuery1" true)))
  (:`Started`
    (`self.SetMapMarkerLocation` _location)
    (bind _geographiccoordinates (`GeoReferencingSystem.EngineToGeographic` (`GeoReferencingSystem.GetGeoReferencingSystem`) _location))
    (bind (_longitude _latitude) (break `GeographicCoordinates` _geographiccoordinates))
    (`EditableText.SetText` (`/Game/WBP_HUDOverlay.Longitude` _hud_overlay) (`KismetTextLibrary.Conv_DoubleToText` _longitude "HalfToEven" false true 1 324 0 10))
    (`EditableText.SetText` (`/Game/WBP_HUDOverlay.Latitude` _hud_overlay) (`KismetTextLibrary.Conv_DoubleToText` _latitude "HalfToEven" false true 1 324 0 10))))

(fn `SetMapMarkerLocation`
  (params (NewLocation :type "Vector Structure"))
  (`self.K2_SetActorLocation` (`self.MapMarker`) NewLocation false false))

(fn `UserConstructionScript`)